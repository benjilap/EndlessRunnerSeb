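; Player for a three-lane runner: a physics cube that moves forward by itself, with Q/D changing lane and A/E turning it in 90-degree steps.
; The orientation index picks force and rotation from arrays built at BeginPlay.
; Tick lerps the cube toward the lane given by the last overlapped PrefabTerrain when axes match.
; It also pushes the cube up to a speed cap, counters sideways drift and prints debug velocity.
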(event EventBeginPlay
  (CallFunction|SetOrientValue)
  (CallFunction|UpdateOrientValue))

(event Collision|EventActorBeginOverlap
  (params (OtherActor :type Actor%20Object%20Reference))
  ;[1 1 1] DetectNewgGround
  (bind _asprefab_terrain (Utilities|Casting|CastToPrefabTerrain OtherActor))
  (bind _output_get (Variables|Default|SetActualTerrain _asprefab_terrain)))

(event EventTick
  (params (DeltaSeconds :type Float%20%28single-precision%29))
  (bind _currentrot (Variables|OrientVar|GetCurrentRot))
  ;[1 1 1] FonctionBehaviour
  (Utilities|FlowControl|Sequence
    (:then_0
      (CallFunction|UpdateLanePlayerPos DeltaSeconds (Variables|Default|GetActualTerrain)))
    (:then_1
      (CallFunction|PlayerMovement))
    (:then_2
      (if (Utilities|Enum|NotEqual(Enum) (Transformation|GetWorldRotation (Variables|Default|GetCube)) _currentrot)
        (Transformation|SetWorldRotation (Variables|Default|GetCube) _currentrot false false)))
    (:then_3
      (CallFunction|UpdateOrientValue))))

(event Input|KeyboardEvents|Q
  (params (Key :type Key%20Structure))
  (bind _playerlane (Variables|Default|GetPlayerLane))
  ;[1 1 1] Input Change lane
  (:Pressed
    (if (> _playerlane 0)
      (Math|Integer|DecrementInt _playerlane))))

(event Input|KeyboardEvents|D
  (params (Key :type Key%20Structure))
  (bind _playerlane (Variables|Default|GetPlayerLane))
  ;[1 1 1] Input Change lane
  (:Pressed
    (if (< _playerlane 2)
      (Math|Integer|IncrementInt _playerlane))))

(event Input|KeyboardEvents|A
  (params (Key :type Key%20Structure))
  ;[1 1 1] Input Change lane
  (:Pressed
    (if (> (Variables|OrientVar|GetOrientValue) 0)
      (Math|Integer|DecrementInt (Variables|OrientVar|GetOrientValue))
      (else
        (Variables|OrientVar|SetOrientValue 3)))))

(event Input|KeyboardEvents|E
  (params (Key :type Key%20Structure))
  ;[1 1 1] Input Change lane
  (:Pressed
    (if (< (Variables|OrientVar|GetOrientValue) 3)
      (Math|Integer|IncrementInt (Variables|OrientVar|GetOrientValue))
      (else
        (Variables|OrientVar|SetOrientValue 0)))))

(fn ConstructionScript)

(fn SetOrientValue
  (bind _moveorigingraph (Variables|OrientVar|GetMoveOriginGraph))
  (bind (_x _y) (Math|Vector|BreakVector _moveorigingraph))
  (Variables|OrientVar|SetForceVector (Utilities|Array|MakeArray (Math|Vector|MakeVector _x 0.0 0.0) (Math|Vector|MakeVector 0.0 _y 0.0) (Math|Vector|MakeVector (* _x -1.0) 0.0 0.0) (Math|Vector|MakeVector 0.0 (* _y -1.0) 0.0)))
  (Variables|OrientVar|SetRotVector (Utilities|Array|MakeArray "0, 0, 0" "0,90.000000,0.000000" "0,180.000000,0.000000" "0,270.000000,0.000000")))

(fn UpdateOrientValue
  (bind _orientvalue (Variables|OrientVar|GetOrientValue))
  (Variables|OrientVar|SetActualForce (Utilities|Array|Get(acopy) (Variables|OrientVar|GetForceVector) _orientvalue))
  (Variables|OrientVar|SetCurrentRot (Utilities|Array|Get(acopy) (Variables|OrientVar|GetRotVector) _orientvalue)))

(fn UpdateLanePlayerPos
  (params (Time :type Float%20%28single-precision%29) (Terrain :type Prefab%20Terrain%20Object%20Reference))
  (bind _playerlane (Variables|Default|GetPlayerLane))
  (bind _laneposition (Variables|/Game/Benji/Prefab/PrefabTerrain.PrefabTerrain_C|GetLanePosition Terrain))
  (bind _cube (Variables|Default|GetCube))
  (bind _cube_2 (Variables|Default|GetCube))
  (bind _playerlane_2 (Variables|Default|GetPlayerLane))
  (bind _laneposition_2 (Variables|/Game/Benji/Prefab/PrefabTerrain.PrefabTerrain_C|GetLanePosition Terrain))
  (bind _orientation (Variables|/Game/Benji/Prefab/PrefabTerrain.PrefabTerrain_C|GetOrientation Terrain))
  (bind _returnvalue (Transformation|GetWorldTransform _cube_2))
  (bind _returnvalue_2 (Transformation|GetWorldTransform _cube))
  (bind _output (Utilities|Array|Get(acopy) _laneposition_2 _playerlane_2))
  (bind _output_2 (Utilities|Array|Get(acopy) _laneposition _playerlane))
  (bind (_location _rotation _scale) (Math|Transform|BreakTransform _returnvalue))
  (bind _location_2 (Math|Transform|BreakTransform _returnvalue_2))
  (bind (_x _y _z) (Math|Vector|BreakVector _location))
  (bind (_x_2 _y_2 _z_2) (Math|Vector|BreakVector _location_2))
  (Utilities|IsValid Terrain
    (:Is%20Valid
      (if (== _orientation 0)
        (if (== (.Y (Math|Vector|BreakVector (Variables|OrientVar|GetActualForce))) 0.0)
          (if (!= _output_2 _y_2)
            (Transformation|SetWorldTransform (Variables|Default|GetCube) (Math|Transform|Lerp(Transform) _returnvalue_2 (Math|Transform|MakeTransform (Math|Vector|MakeVector _x_2 _output_2 _z_2)) (* Time (Variables|Default|GetLaneChangeSpeed))) false false)))
        (elif (== _orientation 1)
          (if (== (.X (Math|Vector|BreakVector (Variables|OrientVar|GetActualForce))) 0.0)
            (if (!= _output _x)
              (Transformation|SetWorldTransform (Variables|Default|GetCube) (Math|Transform|Lerp(Transform) _returnvalue (Math|Transform|MakeTransform (Math|Vector|MakeVector _output _y _z) _rotation _scale) (* Time (Variables|Default|GetLaneChangeSpeed))) false false))))))))

(fn PlayerMovement
  (bind _orientvalue (Variables|OrientVar|GetOrientValue))
  (bind _cube (Variables|Default|GetCube))
  (bind _returnvalue (Transformation|GetComponentVelocity _cube))
  (bind (_x _y) (Math|Vector|BreakVector _returnvalue))
  (bind _returnvalue_2 (Utilities|String|ToString(Float) _y))
  (bind _returnvalue_3 (Utilities|String|ToString(Float) _x))
  (bind _returnvalue_4 (Utilities|String|ToString(Float) _x))
  (bind _returnvalue_5 (Utilities|String|ToString(Float) _y))
  (Utilities|FlowControl|Sequence
    (:then_0
      (if (== _orientvalue 0)
        (Utilities|FlowControl|Sequence
          (:then_0
            (if (<= _x 3e+02) :!label _label
              (Development|PrintString _returnvalue_4)
              (Physics|AddForce _cube (Variables|OrientVar|GetActualForce) "None" false :!label _label_2)
              (else
                (Development|PrintString _returnvalue_4))))
          (:then_1
            (if (!= _y 0.0)
              (Physics|AddForce _cube (- (Math|Vector|MakeVector _x 0.0 0.0) _returnvalue) "None" false)
              (goto _label))))))
    (:then_1
      (if (== _orientvalue 1)
        (Utilities|FlowControl|Sequence
          (:then_0
            (if (<= _y 3e+02) :!label _label_3
              (Development|PrintString _returnvalue_2)
              (goto _label_2)
              (else
                (Development|PrintString _returnvalue_2))))
          (:then_1
            (if (!= _x 0.0)
              (Physics|AddForce _cube (- (Math|Vector|MakeVector 0.0 _y 0.0) _returnvalue) "None" false)
              (goto _label_3))))))
    (:then_2
      (if (== _orientvalue 2)
        (Utilities|FlowControl|Sequence
          (:then_0
            (if (>= _x -3e+02) :!label _label_4
              (Development|PrintString _returnvalue_3)
              (goto _label_2)
              (else
                (Development|PrintString _returnvalue_3))))
          (:then_1
            (if (!= _y 0.0)
              (Physics|AddForce _cube (- (Math|Vector|MakeVector _x 0.0 0.0) _returnvalue) "None" false)
              (goto _label_4))))))
    (:then_3
      (if (== _orientvalue 3)
        (Utilities|FlowControl|Sequence
          (:then_0
            (if (>= _y -3e+02) :!label _label_5
              (Development|PrintString _returnvalue_5)
              (goto _label_2)
              (else
                (Development|PrintString _returnvalue_5))))
          (:then_1
            (if (!= _x 0.0)
              (Physics|AddForce _cube (- (Math|Vector|MakeVector 0.0 _y 0.0) _returnvalue) "None" false)
              (goto _label_5))))))))