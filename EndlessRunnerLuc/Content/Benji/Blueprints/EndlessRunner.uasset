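; Endless runner manager that builds the track, tracks player death and score, and revives the player.
; Tick drops passed segments and spawns new ones, turning randomly left or right after random-length straights and clearing obstacles around corners.
; Straights get random-lane barriers or metro cars with self-adjusting odds, plus chance-based power-ups.
; On death it inserts the score into the saved leaderboard and shows the game-over widget.
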(event Custom|InitGame
  ;[1 1 1] Init Game
  (for _index (range 0 (Variables|Init|GetInitTerrainNum))
    (bind _returnvalue (Game|SpawnActorfromClass "/Game/Benji/Prefab/PrefabTerrain.PrefabTerrain_C" (Variables|SpawnTransformSet|GetNextTransform) "Undefined" 0 0))
    (if (Utilities|Array|IsValidIndex (Variables|SpawnTransformSet|GetPositions))
      _
      (else
        (CallFunction|SetOrientValue _returnvalue)))
    (Utilities|Array|Add (Variables|RoadList|GetActualsRoads) _returnvalue)
    (Variables|SpawnTransformSet|SetNextTransform (Math|Transform|MakeTransform (+ (Utilities|Array|Get(acopy) (Variables|SpawnTransformSet|GetPositions) (Variables|SpawnTransformSet|GetRoadOrientation)) (Transformation|GetWorldLocation (Variables|/Game/Benji/Prefab/PrefabTerrain.PrefabTerrain_C|GetDefaultSceneRoot _returnvalue))) (Math|Rotator|MakeRotator (Utilities|Array|Get(acopy) (Variables|SpawnTransformSet|GetOrientation) (Variables|SpawnTransformSet|GetRoadOrientation)) 0.0 0.0)))))

(event EventBeginPlay
  (Input|SetInputModeGameandUI (Game|GetPlayerController 0) 0 "DoNotLock" true)
  (CallFunction|AddPlayerWidget)
  (CallFunction|InitGame)
  (Variables|BonusData|SetChanceToSpawn (Variables|BonusData|GetBonusPourcentSpawn)))

(event EventTick
  (params (DeltaSeconds :type Float%20%28single-precision%29))
  (Utilities|FlowControl|Sequence
    (:then_0
      (CallFunction|GetPlayerScore)
      (bind _asbp_player (Utilities|Casting|CastToBP_Player (Game|Player|GetPlayerPawn 0)))
      (if (Variables|/Game/Benji/Prefab/BP_Player.BP_Player_C|GetPlayerIsDead _asbp_player)
        (Utilities|FlowControl|DoOnce false :!label _label
          (:Completed
            (CallFunction|LoadSavedStats)))
        (else
          (goto _label Reset))))
    (:then_1
      (CallFunction|CheckRoads)
      (CallFunction|SpawnNewRoads)
      (CallFunction|ResetObsAftTurn))))

(fn ConstructionScript)

(fn SetOrientValue
  (params (MyFirstTerrain :type Prefab%20Terrain%20Object%20Reference))
  (bind _box (Variables|/Game/Benji/Prefab/PrefabTerrain.PrefabTerrain_C|GetBox MyFirstTerrain))
  (bind _boxextent (Variables|/Script/Engine.BoxComponent|GetBoxExtent _box))
  (bind (_x _y) (Math|Vector|BreakVector _boxextent))
  (Variables|SpawnTransformSet|SetOrientation (Utilities|Array|MakeArray 0.0 9e+01 1.8e+02 2.7e+02))
  (Variables|SpawnTransformSet|SetLeftCornerOrientation (Utilities|Array|MakeArray 0.0 9e+01 1.8e+02 2.7e+02))
  (Variables|SpawnTransformSet|SetRightCornerOrientation (Utilities|Array|MakeArray 1.8e+02 2.7e+02 0.0 9e+01))
  (Variables|SpawnTransformSet|SetPositions (Utilities|Array|MakeArray (Math|Vector|MakeVector (* _x 2.0) 0.0 0.0) (Math|Vector|MakeVector 0.0 (* _y 2.0) 0.0) (Math|Vector|MakeVector (* _x -2.0) 0.0 0.0) (Math|Vector|MakeVector 0.0 (* _y -2.0) 0.0)))
  (Variables|SpawnTransformSet|SetRoadOrientation 0))

(fn CheckRoads
  (bind _actualsroads (Variables|RoadList|GetActualsRoads))
  (for (_array_element _array_index) _actualsroads
    (if (Variables|/Game/Benji/Prefab/PrefabTerrain.PrefabTerrain_C|GetBetouched _array_element)
      (if (Utilities|Array|IsValidIndex _actualsroads)
        (bind _output_get (LocalVariables|SetLastRoad (Utilities|Array|Get(acopy) _actualsroads))))
      (if (== _array_index 2)
        (for _array_element_2 (Actor|GetAttachedActors _output_get)
          (Actor|DestroyActor _array_element_2))
        (Actor|DestroyActor _output_get)
        (Utilities|Array|RemoveIndex _actualsroads)))))

(fn SpawnNewRoads
  (if (< (Utilities|Array|Length (Variables|RoadList|GetActualsRoads)) (Variables|Init|GetNumOfTerrain))
    (bind _returnvalue (Game|SpawnActorfromClass "/Game/Benji/Prefab/PrefabTerrain.PrefabTerrain_C" (Variables|SpawnTransformSet|GetNextTransform) "Undefined" 0 0))
    (if (Utilities|Array|IsValidIndex (Variables|SpawnTransformSet|GetPositions))
      _
      (else
        (CallFunction|SetOrientValue _returnvalue)))
    (Utilities|Array|Add (Variables|RoadList|GetActualsRoads) _returnvalue)
    (Math|Integer|DecrementInt (Variables|Init|GetNumToNextCorn)
      (:%20%20
        (if (> (Variables|Init|GetNumToNextCorn) 0)
          (Utilities|FlowControl|Sequence
            (:then_0
              (Utilities|FlowControl|DoOnce false :!label _label
                (:Completed
                  (bind _obsindex (CallFunction|SetObstacle _returnvalue))
                  (CallFunction|SpawnBonus _obsindex _returnvalue)
                  (Variables|SpawnTransformSet|SetNextTransform (Math|Transform|MakeTransform (+ (Utilities|Array|Get(acopy) (Variables|SpawnTransformSet|GetPositions) (Variables|SpawnTransformSet|GetRoadOrientation)) (Transformation|GetWorldLocation (Variables|/Game/Benji/Prefab/PrefabTerrain.PrefabTerrain_C|GetDefaultSceneRoot _returnvalue))) (Math|Rotator|MakeRotator 0.0 0.0 (Utilities|Array|Get(acopy) (Variables|SpawnTransformSet|GetOrientation) (Variables|SpawnTransformSet|GetRoadOrientation)))) :!label _label_2)
                  (Variables|/Game/Benji/Prefab/PrefabTerrain.PrefabTerrain_C|SetRoadOrient _returnvalue (Variables|SpawnTransformSet|GetRoadOrientation)))))
            (:then_1
              (if (not (== (- (Variables|Init|GetNumToNextCorn) 1) 0))
                (goto _label Reset))))
          (else
            (Variables|/Game/Benji/Prefab/PrefabTerrain.PrefabTerrain_C|SetRoadType _returnvalue 1)
            (Default|SetRoadType _returnvalue)
            (if (>= (Math|Random|RandomFloatinRange 0.0 1.0) 0.5)
              (Transformation|SetActorTransform _returnvalue (Math|Transform|MakeTransform (.Location (Math|Transform|BreakTransform (Transformation|GetActorTransform _returnvalue))) (Math|Rotator|MakeRotator 0.0 0.0 (Utilities|Array|Get(acopy) (Variables|SpawnTransformSet|GetRightCornerOrientation) (Variables|SpawnTransformSet|GetRoadOrientation)))))
              (if (< (Variables|SpawnTransformSet|GetRoadOrientation) 3)
                (Math|Integer|IncrementInt (Variables|SpawnTransformSet|GetRoadOrientation)
                  (:%20%20
                    _))
                (else
                  (Variables|SpawnTransformSet|SetRoadOrientation 0)))
              (else
                (if (> (Variables|SpawnTransformSet|GetRoadOrientation) 0)
                  (Math|Integer|DecrementInt (Variables|SpawnTransformSet|GetRoadOrientation)
                    (:%20%20
                      _))
                  (else
                    (Variables|SpawnTransformSet|SetRoadOrientation 3)))
                (Transformation|SetActorTransform _returnvalue (Math|Transform|MakeTransform (.Location (Math|Transform|BreakTransform (Transformation|GetActorTransform _returnvalue))) (Math|Rotator|MakeRotator 0.0 0.0 (Utilities|Array|Get(acopy) (Variables|SpawnTransformSet|GetLeftCornerOrientation) (Variables|SpawnTransformSet|GetRoadOrientation)))))))
            (Variables|Init|SetNumToNextCorn (Math|Random|RandomIntegerinRange 5 10))
            (Default|ResetObstacle _returnvalue)
            (goto _label_2)))))))

(fn AddPlayerWidget
  (bind _returnvalue (UserInterface|CreateWidget "/Game/Benji/Blueprints/PlayerWidget.PlayerWidget_C"))
  (UserInterface|Viewport|AddtoViewport _returnvalue 0))

(fn GetPlayerScore
  (bind _asbp_player (Utilities|Casting|CastToBP_Player (Game|Player|GetPlayerPawn 0)))
  (Variables|ScoreBoardData|SetActualPlayerScore (Variables|/Game/Benji/Prefab/BP_Player.BP_Player_C|GetPlayerScore _asbp_player)))

(fn LoadSavedStats
  (bind _returnvalue (Game|GetPlayerController 0))
  (bind _tempscoreboarddata (Variables|ScoreBoardData|GetTempScoreBoardData))
  (bind _actualplayerscore (Variables|ScoreBoardData|GetActualPlayerScore))
  (bind _asendless_runner_game_instance (Utilities|Casting|CastToEndlessRunnerGameInstance (Game|GetGameInstance)))
  (bind _returnvalue_2 (SaveGame|LoadGamefromSlot "SaveGameScore"))
  (bind _assave_game_score (Utilities|Casting|CastToSaveGameScore _returnvalue_2)
    (:then
      (for _array_element (Variables|/Game/Benji/Blueprints/SaveGameScore.SaveGameScore_C|GetPlayersScore _assave_game_score)
        (Utilities|FlowControl|Sequence
          (:then_0
            (if (<= (.playerScore (Utilities|Struct|BreakplayerScore _array_element)) _actualplayerscore)
              (Utilities|FlowControl|DoOnce false
                (:Completed
                  (Utilities|Array|Add _tempscoreboarddata (Utilities|Struct|MakeplayerScore (Variables|/Game/Benji/Blueprints/EndlessRunnerGameInstance.EndlessRunnerGameInstance_C|GetCurrentPlayerName _asendless_runner_game_instance) _actualplayerscore))))))
          (:then_1
            (Utilities|Array|Add _tempscoreboarddata _array_element))))
      (Utilities|FlowControl|Sequence
        (:then_0
          (Utilities|FlowControl|DoOnce false :!label _label
            (:Completed
              (Utilities|Array|Add _tempscoreboarddata (Utilities|Struct|MakeplayerScore (Variables|/Game/Benji/Blueprints/EndlessRunnerGameInstance.EndlessRunnerGameInstance_C|GetCurrentPlayerName _asendless_runner_game_instance) _actualplayerscore)))))
        (:then_1
          (bind _returnvalue_3 (SaveGame|CreateSaveGameObject "/Game/Benji/Blueprints/SaveGameScore.SaveGameScore_C" :!label _label_2))
          (Variables|/Game/Benji/Blueprints/SaveGameScore.SaveGameScore_C|SetPlayersScore _returnvalue_3 (Variables|ScoreBoardData|GetTempScoreBoardData))
          (SaveGame|SaveGametoSlot _returnvalue_3 "SaveGameScore")
          (bind _returnvalue_4 (UserInterface|CreateWidget "/Game/Benji/Blueprints/GameOverWidget.GameOverWidget_C" _returnvalue (Variables|ScoreBoardData|GetTempScoreBoardData)))
          (UserInterface|Viewport|AddtoViewport _returnvalue_4 0)
          (Variables|/Script/Engine.PlayerController|SetbShowMouseCursor _returnvalue true))))
    (:CastFailed
      (Utilities|FlowControl|Sequence
        (:then_0
          (goto _label))
        (:then_1
          (goto _label_2))))))

(fn SetObstacle
  (params (SpawnedTerrain :type Prefab%20Terrain%20Object%20Reference))
  (bind _obs_barrier (Variables|/Game/Benji/Prefab/PrefabTerrain.PrefabTerrain_C|GetObs_Barrier SpawnedTerrain))
  (bind _obs_metrocar (Variables|/Game/Benji/Prefab/PrefabTerrain.PrefabTerrain_C|GetObs_MetroCar SpawnedTerrain))
  (bind _lftroad (Variables|/Game/Benji/Prefab/PrefabTerrain.PrefabTerrain_C|GetLftRoad SpawnedTerrain))
  (bind _midroad (Variables|/Game/Benji/Prefab/PrefabTerrain.PrefabTerrain_C|GetMidRoad SpawnedTerrain))
  (bind _rhtroad (Variables|/Game/Benji/Prefab/PrefabTerrain.PrefabTerrain_C|GetRhtRoad SpawnedTerrain))
  (bind _array (Utilities|Array|MakeArray _lftroad _midroad _rhtroad))
  (bind _returnvalue (Utilities|Array|Length _array))
  (bind _returnvalue_2 (- _returnvalue 1))
  (bind _returnvalue_3 (Math|Random|RandomIntegerinRange 0 _returnvalue_2))
  (bind _output (Utilities|Array|Get(acopy) _array _returnvalue_3))
  (bind _relativelocation (Variables|/Script/Engine.SceneComponent|GetRelativeLocation _output))
  (if (< (Math|Random|RandomFloat) (LocalVariables|GetBarrier_Chance))
    (Rendering|SetVisibility _obs_barrier true true)
    (LocalVariables|SetBarrier_Chance (- (LocalVariables|GetBarrier_Chance) 0.05))
    (Transformation|SetRelativeLocation _obs_barrier _relativelocation false false)
    (else
      (Rendering|SetVisibility _obs_metrocar true true)
      (LocalVariables|SetBarrier_Chance (+ (LocalVariables|GetBarrier_Chance) 0.2))
      (Transformation|SetRelativeLocation _obs_metrocar _relativelocation false false)))
  (return _output))

(fn SpawnBonus
  (params (ObsLane :type Scene%20Component%20Object%20Reference) (SpawnedRoad :type Prefab%20Terrain%20Object%20Reference))
  (bind _bonuspourcentspawn (Variables|BonusData|GetBonusPourcentSpawn))
  (bind _output_get (LocalVariables|SetSpawnLocation (Utilities|Array|MakeArray (Variables|/Game/Benji/Prefab/PrefabTerrain.PrefabTerrain_C|GetLftRoad SpawnedRoad) (Variables|/Game/Benji/Prefab/PrefabTerrain.PrefabTerrain_C|GetMidRoad SpawnedRoad) (Variables|/Game/Benji/Prefab/PrefabTerrain.PrefabTerrain_C|GetRhtRoad SpawnedRoad))))
  (Utilities|Array|RemoveItem _output_get ObsLane)
  (if (<= (Math|Random|RandomFloat) (Variables|BonusData|GetChanceToSpawn))
    (bind _returnvalue (Game|SpawnActorfromClass "/Game/Benji/Prefab/PowerUp.PowerUp_C" (Math|Transform|MakeTransform (+ (Transformation|GetWorldLocation (Utilities|Array|Get(acopy) (LocalVariables|GetSpawnLocation) (Math|Random|RandomIntegerinRange 0 (- (Utilities|Array|Length (LocalVariables|GetSpawnLocation)) 1)))) "0, 0,80.000000")) "AlwaysSpawn" 0 0))
    (if (or (Class|PrimitiveComponent|IsOverlappingComponent (Variables|/Game/Benji/Prefab/PowerUp.PowerUp_C|GetPickUp_Trigger _returnvalue) (Variables|/Game/Benji/Prefab/PrefabTerrain.PrefabTerrain_C|GetBarrier_Trigger SpawnedRoad)) (Class|PrimitiveComponent|IsOverlappingComponent (Variables|/Game/Benji/Prefab/PowerUp.PowerUp_C|GetPickUp_Trigger _returnvalue) (Variables|/Game/Benji/Prefab/PrefabTerrain.PrefabTerrain_C|GetMetroCar_Trigger SpawnedRoad)))
      (Actor|DestroyActor _returnvalue)
      (Variables|BonusData|SetChanceToSpawn (+ (Variables|BonusData|GetChanceToSpawn) 0.1))
      (else
        (if (> (Variables|BonusData|GetChanceToSpawn) _bonuspourcentspawn)
          (Variables|BonusData|SetChanceToSpawn _bonuspourcentspawn))
        (Transformation|AttachComponentToComponent (Variables|/Script/Engine.Actor|GetRootComponent _returnvalue) (Utilities|Array|Get(acopy) (LocalVariables|GetSpawnLocation) (Math|Random|RandomIntegerinRange 0 (- (Utilities|Array|Length (LocalVariables|GetSpawnLocation)) 1))) "None" "KeepWorld" "KeepRelative" "KeepRelative" true)))))

(fn ResetObsAftTurn
  (bind _actualsroads (Variables|RoadList|GetActualsRoads))
  (for (_array_element _array_index) _actualsroads
    (Utilities|IsValid (Utilities|Array|Get(acopy) _actualsroads (- _array_index 1))
      (:Is%20Valid
        (if (== (Variables|/Game/Benji/Prefab/PrefabTerrain.PrefabTerrain_C|GetRoadType (Utilities|Array|Get(acopy) _actualsroads (- _array_index 1))) 1)
          (Default|ResetObstacle _array_element))))))

(fn RevivePlayer
  (bind _actualsroads (Variables|RoadList|GetActualsRoads))
  (bind _asbp_player (Utilities|Casting|CastToBP_Player (Game|Player|GetPlayerPawn 0)))
  (if (== (Variables|/Game/Benji/Prefab/PrefabTerrain.PrefabTerrain_C|GetRoadType (Variables|/Game/Benji/Prefab/BP_Player.BP_Player_C|GetActualTerrain _asbp_player)) 0)
    (bind _output_get (LocalVariables|SetRestartRoad (Variables|/Game/Benji/Prefab/BP_Player.BP_Player_C|GetActualTerrain _asbp_player)))
    (for _index (range (Utilities|Array|FindItem _actualsroads _output_get) (+ (Utilities|Array|FindItem _actualsroads _output_get) 2))
      (Default|ResetObstacle (Utilities|Array|Get(acopy) _actualsroads _index)))
    (else
      (bind _output_get_2 (LocalVariables|SetRestartRoad (Utilities|Array|Get(acopy) _actualsroads (+ (Utilities|Array|FindItem _actualsroads (Variables|/Game/Benji/Prefab/BP_Player.BP_Player_C|GetActualTerrain _asbp_player)) 1))))
      (for _index_2 (range (Utilities|Array|FindItem _actualsroads _output_get_2) (+ (Utilities|Array|FindItem _actualsroads _output_get_2) 2))
        (Default|ResetObstacle (Utilities|Array|Get(acopy) _actualsroads _index_2)))))
  (Variables|/Game/Benji/Prefab/BP_Player.BP_Player_C|SetHadRevive _asbp_player false)
  (Variables|/Game/Benji/Prefab/BP_Player.BP_Player_C|SetPlayerIsDead _asbp_player false)
  (Transformation|SetWorldLocation (Variables|/Game/Benji/Prefab/BP_Player.BP_Player_C|GetCarMesh _asbp_player) (Math|Vector|MakeVector (.X (Math|Vector|BreakVector (Transformation|GetWorldLocation (Variables|/Game/Benji/Prefab/PrefabTerrain.PrefabTerrain_C|GetDefaultSceneRoot (LocalVariables|GetRestartRoad))))) (.Y (Math|Vector|BreakVector (Transformation|GetWorldLocation (Variables|/Game/Benji/Prefab/PrefabTerrain.PrefabTerrain_C|GetDefaultSceneRoot (LocalVariables|GetRestartRoad))))) (.Z (Math|Vector|BreakVector (Transformation|GetWorldLocation (Variables|/Game/Benji/Prefab/BP_Player.BP_Player_C|GetCarMesh _asbp_player))))) false false)
  (Variables|/Game/Benji/Prefab/BP_Player.BP_Player_C|SetOrientValue _asbp_player (Variables|/Game/Benji/Prefab/PrefabTerrain.PrefabTerrain_C|GetRoadOrient (LocalVariables|GetRestartRoad)))
  (bind _foundwidgets (Widget|GetAllWidgetsOfClass "/Game/Benji/Blueprints/GameOverWidget.GameOverWidget_C" true))
  (for _array_element _foundwidgets
    (Widget|RemovefromParent _array_element)))